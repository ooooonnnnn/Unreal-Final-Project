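; BP_Reticle_Aiming computes the world point the player is aiming at through an on-screen crosshair.
; On BeginPlay it creates the WB_HUD widget and keeps its Crosshair element.
; Each tick it deprojects the crosshair's viewport center into a world ray and runs a Visibility line trace out to PlayerAimDistance.
; PlayerAimTarget becomes the hit location, or the ray's end point when nothing blocks.
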(event `self.ReceiveBeginPlay`
  (bind _returnvalue (`|CreateWidget` "/Game/Blueprints/UI/HUD/WB_HUD.WB_HUD_C" (`GameplayStatics.GetPlayerController` 0)))
  (`UserWidget.AddToViewport` _returnvalue 0)
  (set `self.Crosshair` (`/Game/Blueprints/UI/HUD/WB_HUD.Crosshair` _returnvalue)))

(event `self.ReceiveTick`
  (params (DeltaSeconds :type "Float (single-precision)"))
  (bind _returnvalue (`Widget.GetTickSpaceGeometry` (`self.Crosshair`)))
  (bind (_worldposition _worlddirection) (`GameplayStatics.DeprojectScreenToWorld` (`GameplayStatics.GetPlayerController` 0) (`SlateBlueprintLibrary.LocalToViewport` _returnvalue (/ (`SlateBlueprintLibrary.GetLocalSize` _returnvalue) 2.0))))
  (bind _returnvalue_2 (+ _worldposition (* _worlddirection (`self.Player Aim distance`))))
  ;[1 1 1] Ray cast to find player aim position
  (bind _outhit (`KismetSystemLibrary.LineTraceSingle` _worldposition _returnvalue_2 "TraceTypeQuery1"))
  (if (`GameplayStatics.BreakHitResult` _outhit)
    (set `self.Player Aim Target` (`.Location` (`GameplayStatics.BreakHitResult` _outhit)))
    (else
      (set `self.Player Aim Target` _returnvalue_2))))