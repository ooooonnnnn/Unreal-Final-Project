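; BP_Circle_Creator is an actor that spawns copies of BaseActor in a horizontal ring around its own location.
; CreateCircle steps an angle up to a full turn, rotating a radius vector around Z to place each copy, yawed by that angle plus an offset.
; MaxNumIterations caps the loop, but NumIterations is never reset here, so the count carries across calls.
; The event graph and construction script are empty, so nothing in the file calls CreateCircle.
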(fn `Create circle`
  (set `self.Current Angle` 0.0)
  (while (and (< (`self.Current Angle`) 360.0) (< (`self.Num iterations`) (`self.Max num iterations`)))
    (`|SpawnActorFromClass` (`self.Base actor`) (`KismetMathLibrary.MakeTransform` (+ (`self.K2_GetActorLocation`) (* (`self.Radius`) (`KismetMathLibrary.RotateAngleAxis` (1.0 0.0 0.0) (`self.Current Angle`) (0.0 0.0 1.0)))) (`KismetMathLibrary.MakeRotator` 0.0 0.0 (+ (`self.Current Angle`) (`self.Object Additional Rotation`)))) "AlwaysSpawn" "MultiplyWithRoot" null null)
    (set `self.Current Angle` (+ (`self.Current Angle`) (`self.Angle Step`)))
    (`/Engine/EditorBlueprintResources/StandardMacros.IncrementInt` (`self.Num iterations`))))

(fn `UserConstructionScript`)