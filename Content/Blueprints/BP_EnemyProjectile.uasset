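; BP_EnemyProjectile is an enemy projectile actor that stands in for a randomly chosen elemental spell.
; On BeginPlay it picks a random entry from SpellElements and switches on Fire, Ice or Lightning to spawn the matching test fireball, iceball or electricball Blueprint.
; Each branch has its own spawn transform and always spawns regardless of collision.
; The construction script only calls its parent.
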(event `self.ReceiveBeginPlay`
  (switch `/Game/Blueprints/Enums/E_SpellElements` (`KismetArrayLibrary.Array_Random` (`self.SpellElements`))
    (:`NewEnumerator0`
      (`|SpawnActorFromClass` "/Game/BP_Test_Fireball.BP_Test_Fireball_C" (`self.Spawn Transform_2`) "AlwaysSpawn" "MultiplyWithRoot" null null))
    (:`NewEnumerator1`
      (`|SpawnActorFromClass` "/Game/BP_Test_Iceball.BP_Test_Iceball_C" (`self.Spawn Transform_3`) "AlwaysSpawn" "MultiplyWithRoot" null null))
    (:`NewEnumerator2`
      (`|SpawnActorFromClass` "/Game/BP_Test_Electricball.BP_Test_Electricball_C" (`self.Spawn Transform_4`) "AlwaysSpawn" "MultiplyWithRoot" null null))))

(fn `UserConstructionScript`
  (`parent.UserConstructionScript`))