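; BP_EnemyAI is a spellcasting enemy driven by a Tick-based state machine with Idle, Casting, Defending and Repositioning states.
; Idle traces from head to player, switching to Casting on any hit, otherwise Repositioning.
; Casting uses a DoOnce-guarded delay to spawn a projectile at the right forearm, then repositions via an empty RepositionAI stub.
; Player projectiles entering the sphere trigger Defending, which spawns a wall after an animation if mana suffices.
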(event `self.ReceiveTick`
  (params (DeltaSeconds :type "Float (single-precision)"))
  (switch `/Game/Enums/E_AIState` (`self.CurrentState`)
    (:`NewEnumerator0`
      ; Idle
      (bind (_outhit _returnvalue) (`KismetSystemLibrary.LineTraceSingle` :`Start` (`SceneComponent.GetSocketLocation` (`self.SkeletalMesh`) "Head") :`End` (`self.K2_GetActorLocation` (`GameplayStatics.GetPlayerPawn` 0)) :`TraceChannel` "TraceTypeQuery1" :`DrawDebugType` "Persistent"))
      (if _returnvalue
        (set `self.CurrentState` "NewEnumerator1")
        (else
          (set `self.CurrentState` "NewEnumerator3"))))
    (:`NewEnumerator1`
      ; Casting
      (`/Engine/EditorBlueprintResources/StandardMacros.DoOnce` false :!label _label
        (:`Completed`
          (`KismetSystemLibrary.Delay` 1.2)
          (`|SpawnActorFromClass` "/Game/Blueprints/BP_EnemyProjectile.BP_EnemyProjectile_C" (`SkinnedMeshComponent.GetBoneTransform` (`self.SkeletalMesh`) "RightForeArm" "RTS_World") "Undefined" "MultiplyWithRoot" null null)
          (set `self.CurrentState` "NewEnumerator3")
          (goto _label :!via `Reset`))))
    (:`NewEnumerator2`
      (if (`self.HasEnoughMana`)
        (`SkeletalMeshComponent.PlayAnimation` (`self.SkeletalMesh`) null false)
        (`KismetSystemLibrary.Delay` 1.2)
        (`|SpawnActorFromClass` "/Game/Blueprints/BP_Wall.BP_Wall_C" (`self.Spawn Transform`) "Undefined" "MultiplyWithRoot" null null)
        (`KismetSystemLibrary.Delay` 0.2)
        (set `self.CurrentState` "NewEnumerator0")))
    (:`NewEnumerator3`
      (`self.RepositionAI`))))

(event `self.Sphere.OnComponentBeginOverlap`
  (params (OverlappedComponent :type "PrimitiveComponent Object Reference") (OtherActor :type "Actor Object Reference") (OtherComp :type "PrimitiveComponent Object Reference") (OtherBodyIndex :type Integer) (bFromSweep :type Boolean) (SweepResult :type "HitResult Structure (by ref)"))
  (cast `/Game/Blueprints/BP_PlayerProjectile` OtherActor)
  (set `self.CurrentState` "NewEnumerator2"))

(fn `RepositionAI`)

(fn `UserConstructionScript`)