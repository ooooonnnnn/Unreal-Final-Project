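; BP_Character is a character Blueprint with a cooldown-limited dodge.
; BeginPlay adds the IMC_Game Enhanced Input mapping context.
; The Dodge event checks and clears CanDodge, calls PerformDodge, then restores the flag after a delay.
; PerformDodge instantly offsets the actor horizontally by a set distance along its last movement direction, sweeping for collision rather than applying an impulse.
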(event `self.ReceiveBeginPlay`
  (`EnhancedInputSubsystemInterface.AddMappingContext` (subsystem `EnhancedInputLocalPlayerSubsystem`) "/Game/Input/IMC_Game.IMC_Game" 0 (struct)))

(event `Dodge`
  (if (`self.Can Dodge`)
    (`|ExecutionSequence`
      (:`then_0`
        (set `self.Can Dodge` false))
      (:`then_1`
        (`self.Perform Dodge`)
        (`KismetSystemLibrary.Delay` (`self.Dodge Cooldown`))
        (set `self.Can Dodge` true)))))

(fn `Perform Dodge`
  (`self.K2_AddActorWorldOffset` (`KismetMathLibrary.Conv_Vector2DToVector` (* (`KismetMathLibrary.ToDirectionAndLength2D` (`KismetMathLibrary.Conv_VectorToVector2D` (`CharacterMovementComponent.GetLastUpdateVelocity` (`self.CharacterMovement`)))) (`self.Dodge Distance`))) true))

(fn `UserConstructionScript`)