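; BP_Spell_Utils is a set of helper functions for the spell system's three elements: Fire, Ice and Lightning.
; Two lookups define a cyclic strength relationship, returning the element weaker or stronger than a given one.
; The others map each element to its material, Niagara effect, cast sound and destroy sound.
; Every function is a single stateless Select on the element, with assets hardcoded in the Blueprint.
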(fn `Get Cast Sound For Element`
  (params (Element :type "/Game/Blueprints/Enums/E_Element Enum" :default "NewEnumerator0"))
  (returns (`Sound Effect` :type "SoundBase Object Reference"))
  (return (select `/Game/Blueprints/Enums/E_Element` Element :`NewEnumerator0` "/Game/Sounds/Sound_Cues/Magic_Cast/SC_Fire_Cast.SC_Fire_Cast" :`NewEnumerator1` "/Game/Sounds/Sound_Cues/Magic_Cast/SC_Ice_Cast.SC_Ice_Cast" :`NewEnumerator2` "/Game/Sounds/Sound_Cues/Magic_Cast/SC_Electric_Cast.SC_Electric_Cast" :!type "SoundBase Object Reference")))

(fn `Get Destroy Sound For Element`
  (params (Element :type "/Game/Blueprints/Enums/E_Element Enum" :default "NewEnumerator0"))
  (returns (`Sound Effect` :type "SoundBase Object Reference"))
  (return (select `/Game/Blueprints/Enums/E_Element` Element :`NewEnumerator0` "/Game/Sounds/Sound_Cues/Magic_Impact/SC_Fire_Impact.SC_Fire_Impact" :`NewEnumerator1` "/Game/Sounds/Sound_Cues/Magic_Impact/SC_Ice_Impact.SC_Ice_Impact" :`NewEnumerator2` "/Game/Sounds/Sound_Cues/Magic_Impact/SC_Lightning_Impact.SC_Lightning_Impact" :!type "SoundBase Object Reference")))

(fn `Get Material For Element`
  (params (Element :type "/Game/Blueprints/Enums/E_Element Enum" :default "NewEnumerator0"))
  (returns (Material :type "MaterialInterface Object Reference"))
  (return (select `/Game/Blueprints/Enums/E_Element` Element :`NewEnumerator0` "/Game/Materials/M_Burnt.M_Burnt" :`NewEnumerator1` "/Game/Materials/M_Ice.M_Ice" :`NewEnumerator2` "/Game/Materials/M_Electric.M_Electric" :!type "MaterialInterface Object Reference")))

(fn `Get Niagara System For Element`
  (params (Element :type "/Game/Blueprints/Enums/E_Element Enum" :default "NewEnumerator0"))
  (returns (`Idle System` :type "NiagaraSystem Object Reference"))
  (return (select `/Game/Blueprints/Enums/E_Element` Element :`NewEnumerator0` "/Game/Niagara_Systems/NS_Fire.NS_Fire" :`NewEnumerator1` "/Game/Niagara_Systems/NS_IceMist.NS_IceMist" :`NewEnumerator2` "/Game/Niagara_Systems/NS_Lightning.NS_Lightning" :!type "NiagaraSystem Object Reference")))

(fn `Get Stronger Element`
  (params (`Test element` :type "/Game/Blueprints/Enums/E_Element Enum" :default "NewEnumerator0"))
  (returns (`Stronger element` :type "/Game/Blueprints/Enums/E_Element Enum"))
  (return (select `/Game/Blueprints/Enums/E_Element` `Test element` :`NewEnumerator0` "NewEnumerator2" :`NewEnumerator1` "NewEnumerator0" :`NewEnumerator2` "NewEnumerator1" :!type "/Game/Blueprints/Enums/E_Element Enum")))

(fn `Get Weaker Element`
  (params (`Test element` :type "/Game/Blueprints/Enums/E_Element Enum" :default "NewEnumerator0"))
  (returns (`Weaker element` :type "/Game/Blueprints/Enums/E_Element Enum"))
  (return (select `/Game/Blueprints/Enums/E_Element` `Test element` :`NewEnumerator0` "NewEnumerator1" :`NewEnumerator1` "NewEnumerator2" :`NewEnumerator2` "NewEnumerator0" :!type "/Game/Blueprints/Enums/E_Element Enum")))