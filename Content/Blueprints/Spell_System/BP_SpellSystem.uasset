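; BP_SpellSystem handles two-key spell combo input from three spell keys plus a cancel key, and creates the combo UI on BeginPlay.
; The first key is stored and filters the Spells data table by FirstKey, passing matching rows to the widget.
; A second key calls TryCompleteCombo, which is still an empty stub, while cancel only resets the stored key.
; Data table row names are cached in the construction script.
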(event `self.ReceiveBeginPlay`
  (bind _returnvalue (`|CreateWidget` "/Game/Blueprints/UI/WBP_SpellComboUI.WBP_SpellComboUI_C" (`GameplayStatics.GetPlayerController` 0)))
  (`UserWidget.AddToViewport` _returnvalue 0))

(event `Spell_Key1_Event`
  (`self.HandleSpellComboInput` "NewEnumerator1"))

(event `Spell_Key2_Event`
  (`self.HandleSpellComboInput` "NewEnumerator2"))

(event `Spell_Key3_Event`
  (`self.HandleSpellComboInput` "NewEnumerator3"))

(event `Spell_KeyCancel_Event`
  (`self.CancelCombo`))

(fn `CancelCombo`
  (set `self.CurrentFirstKey` "NewEnumerator0"))

(fn `HandleSpellComboInput`
  (params (KeyPressed :type "/Game/Blueprints/Enums/E_ComboKey Enum" :default "NewEnumerator0"))
  (if (`|EnumEquality` (`self.CurrentFirstKey`) "NewEnumerator0")
    (bind _output_get (set `self.CurrentFirstKey` KeyPressed))
    (bind _rowsdata (`self.UpdateSpells` _output_get))
    (`/Game/Blueprints/UI/WBP_SpellComboUI.UpdateSpellTT` (`self.SpellCoboUI`) _rowsdata)
    (else
      (`self.TryCompleteCombo` (`self.CurrentFirstKey`) KeyPressed))))

(fn `TryCompleteCombo`
  (params (CurrentFirstKey :type "/Game/Blueprints/Enums/E_ComboKey Enum" :default "NewEnumerator0") (InputKey :type "/Game/Blueprints/Enums/E_ComboKey Enum" :default "NewEnumerator0")))

(fn `UpdateSpells`
  (params (Key :type "/Game/Blueprints/Enums/E_ComboKey Enum" :default "NewEnumerator0"))
  (returns (RowsData :type "Array of /Game/Blueprints/Structs/ST_SpellData Structure"))
  (locals (SelectedRowsData :type "Array of /Game/Blueprints/Structs/ST_SpellData Structure"))
  (for _array_element (`self.RowNames`)
    (bind _returnvalue (`|GetDataTableRow` (`self.Spells`) _array_element)
      (:`then`
        (if (`|EnumEquality` (`.FirstKey_2_D7D6CBBC40F1A5B8A5DEC7B3AB0BC92A` (break `/Game/Blueprints/Structs/ST_SpellData` _returnvalue)) Key)
          (`KismetArrayLibrary.Array_Add` (`local.SelectedRowsData`) _returnvalue)))))
  (return (`local.SelectedRowsData`)))

(fn `UserConstructionScript`
  (bind _outrownames (`DataTableFunctionLibrary.GetDataTableRowNames` (`self.Spells`)))
  (set `self.RowNames` _outrownames))