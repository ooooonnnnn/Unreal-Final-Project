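; Spell system component that turns two-key input combos into spell selections from the Spells data table.
; On BeginPlay it caches row names and creates the combo UI widget.
; The first key shows matching spells in the UI; the second, which ignores key three, looks up the key pair.
; A match fires OnCompleteCombo with the spell data and resets the combo, as does the cancel key.
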(event `self.ReceiveBeginPlay`
  (bind _outrownames (`DataTableFunctionLibrary.GetDataTableRowNames` (`self.Spells`)))
  (set `self.RowNames` _outrownames)
  (bind _returnvalue (`|CreateWidget` "/Game/Blueprints/UI/SpellUI/WBP_SpellComboUI.WBP_SpellComboUI_C" (`GameplayStatics.GetPlayerController` 0)))
  (bind _output_get (set `self.SpellCoboUI` _returnvalue))
  (`/Game/Blueprints/UI/SpellUI/WBP_SpellComboUI.CreateBaseSpells` _output_get)
  (`UserWidget.AddToViewport` _output_get 0))

(event `Spell_Key1_Event`
  (`self.HandleSpellComboInput` "NewEnumerator1"))

(event `Spell_Key2_Event`
  (`self.HandleSpellComboInput` "NewEnumerator2"))

(event `Spell_Key3_Event`
  (`self.HandleSpellComboInput` "NewEnumerator3"))

(event `Spell_KeyCancel_Event`
  (`self.CancelCombo`))

(fn `CancelCombo`
  (set `self.CurrentFirstKey` "NewEnumerator0")
  (`/Game/Blueprints/UI/SpellUI/WBP_SpellComboUI.ClearCombo` (`self.SpellCoboUI`)))

(fn `HandleSpellComboInput`
  (params (KeyPressed :type "/Game/Blueprints/Enums/E_ComboKey Enum" :default "NewEnumerator0"))
  (if (`|EnumEquality` (`self.CurrentFirstKey`) "NewEnumerator0")
    ;[0.15 0.02578 0.02578 0.5] update UI and first key input
    (bind _output_get (set `self.CurrentFirstKey` KeyPressed))
    (bind _rowsdata (`self.UpdateSpells` _output_get))
    (`/Game/Blueprints/UI/SpellUI/WBP_SpellComboUI.UpdateSpellTT` (`self.SpellCoboUI`) _rowsdata)
    (else
      ;[1 1 1] check if key is 3 that is not exists and skip input
      (if (not (`|EnumEquality` KeyPressed "NewEnumerator3"))
        ;[1 1 1] Try Cast Spell
        (bind (_spell_data _isfound) (`self.TryCompleteCombo` (`self.CurrentFirstKey`) KeyPressed))
        (if _isfound
          (`self.On Complete Combo` _spell_data)
          (`self.CancelCombo`))))))

(fn `TryCompleteCombo`
  (params (CurrentFirstKey :type "/Game/Blueprints/Enums/E_ComboKey Enum" :default "NewEnumerator0") (InputKey :type "/Game/Blueprints/Enums/E_ComboKey Enum" :default "NewEnumerator0"))
  (returns (`Spell Data` :type "/Game/Blueprints/Structs/ST_SpellData Structure") (IsFound :type Boolean))
  (for _array_element (`self.RowNames`)
    (bind _returnvalue (`|GetDataTableRow` (`self.Spells`) _array_element)
      (:`then`
        (bind (_firstkey _secondkey) (break `/Game/Blueprints/Structs/ST_SpellData` _returnvalue))
        (bind _returnvalue_2 (and (`|EnumEquality` _firstkey CurrentFirstKey) (`|EnumEquality` _secondkey InputKey)))
        (if _returnvalue_2
          (return _returnvalue _returnvalue_2)))))
  (return (struct) false))

(fn `UpdateSpells`
  (params (Key :type "/Game/Blueprints/Enums/E_ComboKey Enum" :default "NewEnumerator0"))
  (returns (RowsData :type "Array of /Game/Blueprints/Structs/ST_SpellData Structure"))
  (locals (SelectedRowsData :type "Array of /Game/Blueprints/Structs/ST_SpellData Structure"))
  (for _array_element (`self.RowNames`)
    (bind _returnvalue (`|GetDataTableRow` (`self.Spells`) _array_element)
      (:`then`
        (bind (_firstkey _secondkey _spellclass) (break `/Game/Blueprints/Structs/ST_SpellData` _returnvalue))
        (if (and (`|EnumEquality` _firstkey Key) (!= _spellclass null))
          (`KismetArrayLibrary.Array_Add` (`local.SelectedRowsData`) _returnvalue)))))
  (return (`local.SelectedRowsData`)))