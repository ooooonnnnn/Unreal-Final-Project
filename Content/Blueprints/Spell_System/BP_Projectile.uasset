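; Spell projectile that launches along its launch direction and deals elemental damage to damageable actors it overlaps.
; Overlaps call the I_Damagable interface with element, damage and instigator, skipping the instigator and only printing a warning if none exists.
; It pierces targets whose element is weaker than its own, except one specific element that always stops it.
; Other damaged targets and any non-damageable overlap destroy it.
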(event `self.ReceiveBeginPlay`
  (bind _projectilemovement (`self.ProjectileMovement`))
  (`parent.ReceiveBeginPlay`)
  (set `MovementComponent.Velocity` (* (`self.Launch Direction`) (`ProjectileMovementComponent.InitialSpeed` _projectilemovement)) _projectilemovement))

(event `self.ReceiveActorBeginOverlap`
  (params (OtherActor :type "Actor Object Reference"))
  (bind _returnvalue (`self.GetInstigator`))
  (bind _asi_damagable (cast `/Game/Blueprints/Interfaces/I_Damagable` OtherActor)
    (:`then`
      (`/Engine/EditorBlueprintResources/StandardMacros.IsValid` _returnvalue
        (:`Is Valid`
          (if (not (== OtherActor _returnvalue))
            (`|ExecutionSequence`
              (:`then_0`
                (`/Game/Blueprints/Interfaces/I_Damagable.Recieve Damage` _asi_damagable (`self.Element`) (`self.Damage`) (`self.GetInstigator`)))
              (:`then_1`
                (bind _element (`/Game/Blueprints/Interfaces/I_Damagable.Get Element` _asi_damagable))
                (if (or (not (`/Game/Blueprints/Spell_System/BP_Spell_Utils.Get Strength Relations` _element (`self.Element`))) (`|EnumEquality` _element "NewEnumerator3"))
                  (`self.Event Destroy`))))))
        (:`Is Not Valid`
          (`KismetSystemLibrary.PrintString` "Warning, projectile has no instigator"))))
    (:`CastFailed`
      (`self.Event Destroy`))))

(event `self.ReceiveTick`
  (params (DeltaSeconds :type "Float (single-precision)"))
  (`parent.ReceiveTick` DeltaSeconds))

(fn `UserConstructionScript`
  (`parent.UserConstructionScript`))