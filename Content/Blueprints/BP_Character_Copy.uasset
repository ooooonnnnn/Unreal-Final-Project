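; Player character that casts elemental spells and blinks to dodge, with health and death handled through the game mode.
; CastSpell plays a montage by spell class, slows movement, and spawns a projectile or ground-traced barrier on an anim notify.
; Blinking sweeps the actor along its velocity with Niagara, sound and additive animation feedback, gated by a particle-signalled cooldown.
; Blinking mid-cast cancels the montage through a bound dodge event.
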(event Custom|Event%20Set%20Aim%20Target%20Position
  (params (Target%20Position :type Vector))
  (Collision|LineTraceByChannel (Transformation|GetActorLocation) Target%20Position "TraceTypeQuery1" false 0 "None")
  (Variables|Default|SetTarget%20Position Target%20Position))

(event Custom|Cancel%20animation
  (Animation|StopAnimMontage (Variables|Default|GetSpell%20Cast%20montage)))

(event Custom|Event%20On%20Dodge
  (params (Relative%20direction :type Vector%202D%20Structure) (World%20Direction :type Vector))
  (bind _returnvalue (Transformation|GetActorLocation))
  (Utilities|FlowControl|Sequence
    (:then_0
      (Default|EventBlinkReact (Variables|Default|GetAnimation%20Blueprint) Relative%20direction))
    (:then_1
      (bind _returnvalue_2 (Niagara|SpawnSystematLocation "/Game/Niagara_Systems/NS_Star_Burst_Directional.NS_Star_Burst_Directional" _returnvalue "0, 0, 0" "1.000000,1.000000,1.000000" true false "AutoRelease"))
      (Niagara|SetNiagaraVariable(Vector3) _returnvalue_2 "Direction" World%20Direction)
      (Class|NiagaraFunctionLibrary|OverrideSystemUserVariableSkeletalMeshComponent _returnvalue_2 "Skeletal Mesh" (Variables|Character|GetMesh))
      (Components|Activation|Activate _returnvalue_2 true))
    (:then_2
      (Audio|PlaySoundatLocation "/Game/Sounds/Sound_Cues/SC_Blink.SC_Blink" _returnvalue "0, 0, 0" 1.0 1.0 0.05 0 0 0 0))
    (:then_3
      (Default|CallOnDodge))))

(event Custom|Event%20Die
  (bind _asab_abe (Utilities|Casting|CastToAB_Abe (Components|SkeletalMesh|GetAnimInstance (Variables|Character|GetMesh))))
  (Default|PlayDeathAnimation _asab_abe)
  (Components|Activation|Deactivate (Variables|Character|GetCharacterMovement))
  (Utilities|FlowControl|Delay (Variables|Default|GetDelay%20After%20Death))
  (bind _asbp_game_mode (Utilities|Casting|CastToBP_GameMode (Game|GetGameMode)))
  (Default|EventonPlayerDie _asbp_game_mode))

(event Custom|Event%20Add%20Dodge%20Input
  (if (Variables|Default|GetCan%20Dodge)
    (if (> (Class|KismetMathLibrary|VSize2DSquared (Math|Conversions|ToVector2D(Vector) (Pawn|Components|CharacterMovement|GetLastUpdateVelocity (Variables|Character|GetCharacterMovement)))) 0.0)
      (Utilities|FlowControl|Sequence
        (:then_0
          (Utilities|StartDodgeCooldown))
        (:then_1
          (CallFunction|PerformDodge))
        (:then_2
          (bind _1_to_0 (Timeline|Reaction%20Anim%20Additive%20Weight PlayFromStart)
            (:Update
              (Default|EventUpdateBlinkAdditiveWeight (Variables|Default|GetAnimation%20Blueprint) _1_to_0))))))))

(event Custom|Event%20Cast%20Spell
  (params (Spell%20Data :type ST%20Spell%20Data%20Structure))
  (bind (_firstkey _secondkey _spellclass _spellicon _spellname _spellelement) (Utilities|Struct|BreakST_SpellData Spell%20Data))
  ;[1 1 1] Check spell class
  (Utilities|SwitchonSpellClass _spellclass "/Game/Blueprints/Spell_System/BP_Projectile.BP_Projectile_C" "/Game/Blueprints/Spell_System/BP_Barrier.BP_Barrier_C"
    (:Option%201
      (Variables|Default|SetSpell%20Cast%20montage "/Game/Characters/Abe/Animation/AM_Standing_1H_Magic_Attack_01.AM_Standing_1H_Magic_Attack_01"))
    (:Option%202
      (Variables|Default|SetSpell%20Cast%20montage "/Game/Characters/Abe/Animation/AM_Standing_2H_Cast_Spell_01.AM_Standing_2H_Cast_Spell_01")))
  (bind _notifyname (Animation|Montage|PlayMontage (Variables|Character|GetMesh) (Variables|Default|GetSpell%20Cast%20montage))
    (:then
      ;[1 1 1] Slow down movement
      (Variables|/Script/Engine.CharacterMovementComponent|SetMaxWalkSpeed (Variables|Character|GetCharacterMovement) 1.0)
      ;[1 1 1] Interrupt cast with dodge
      (EventDispatchers|BindEventtoOnDodge (delegate Custom|Cancel%20animation)))
    (:OnCompleted
      (Variables|/Script/Engine.CharacterMovementComponent|SetMaxWalkSpeed (Variables|Character|GetCharacterMovement) (Variables|Default|GetWalk%20Speed) :!label _label)
      (EventDispatchers|UnbindEventfromOnDodge (delegate Custom|Cancel%20animation)))
    (:OnInterrupted
      (goto _label))
    (:OnNotifyBegin
      ;[1 1 1] Cast on notify
      (if (== _notifyname "Action")
        (Utilities|SwitchonSpellClass _spellclass "/Game/Blueprints/Spell_System/BP_Projectile.BP_Projectile_C" "/Game/Blueprints/Spell_System/BP_Barrier.BP_Barrier_C"
          (:Option%201
            (CallFunction|CastProjectile _spellelement))
          (:Option%202
            (CallFunction|CastBarrier _spellelement)))))))

(event EventBeginPlay
  (Utilities|FlowControl|Sequence
    (:then_0
      (Input|AddMappingContext (PlayerController|LocalPlayerSubsystems|GetEnhancedInputLocalPlayerSubsystem) "/Game/Input/IMC_Game.IMC_Game" 0 "(bIgnoreAllPressedKeysUntilRelease=True,bForceImmediately=False,bNotifyUserSettings=False)")
      (bind _asab_abe (Utilities|Casting|CastToAB_Abe (Components|SkeletalMesh|GetAnimInstance (Variables|Character|GetMesh))))
      (Variables|Default|SetAnimation%20Blueprint _asab_abe))
    (:then_1
      (Utilities|StartDodgeCooldown))
    (:then_2
      (Variables|Default|SetWalk%20Speed (Variables|/Script/Engine.CharacterMovementComponent|GetMaxWalkSpeed (Variables|Character|GetCharacterMovement))))))

(event EventRecieveDamage
  (params (Damage%20element :type E_Element%20Enum :default "NewEnumerator0") (Damage%20amount :type Float%20%28double-precision%29))
  (bind _output_get (Variables|Default|SetHealth (- (Variables|Default|GetHealth) Damage%20amount)))
  (if (<= _output_get 0.0)
    (CallFunction|EventDie)))

(event Input|MouseEvents|DebugKeyRightMouseButton
  (params (Key :type Key%20Structure :default "None") (ActionValue :type Input%20Action%20Value%20Structure))
  (:Pressed
    (CallFunction|EventDie)))

(fn ConstructionScript)

(fn PerformDodge
  (bind _charactermovement (Variables|Character|GetCharacterMovement))
  (bind _dodge_distance (Variables|Default|GetDodge%20Distance))
  (bind _returnvalue (Pawn|Components|CharacterMovement|GetLastUpdateVelocity _charactermovement))
  (bind _returnvalue_2 (Math|Conversions|ToVector2D(Vector) _returnvalue))
  (bind _outdir (Class|KismetMathLibrary|ToDirectionandLength2D _returnvalue_2))
  (bind _returnvalue_3 (* _outdir _dodge_distance))
  (bind _returnvalue_4 (Math|Conversions|ToVector(Vector2D) _returnvalue_3))
  (CallFunction|EventonDodge (Math|Conversions|ToVector2D(Vector) (Math|Vector|RotateVector (Math|Conversions|ToVector(Vector2D) _outdir) (Math|Rotator|FindRelativeLookatRotation (Transformation|GetActorTransform self) (+ (Transformation|GetActorLocation) "1.000000,0.000000,0.000000")))) (Math|Vector|Normalize _returnvalue_4))
  (Transformation|AddActorWorldOffset _returnvalue_4 true))

(fn CastProjectile
  (params (Element :type E_Element%20Enum :default "NewEnumerator0"))
  (bind _mesh (Variables|Character|GetMesh))
  (bind _returnvalue (Transformation|GetSocketTransform _mesh "RightHand" "RTS_World"))
  (Game|SpawnActorfromClass "/Game/Blueprints/Spell_System/BP_Projectile.BP_Projectile_C" _returnvalue "AlwaysSpawn" "MultiplyWithRoot" 0 (Math|Vector|Normalize (- (Variables|Default|GetTarget%20Position) (.Location (Math|Transform|BreakTransform _returnvalue)))) Element 0))

(fn CastBarrier
  (params (Element :type E_Element%20Enum :default "NewEnumerator0"))
  (bind _returnvalue (Transformation|GetActorTransform))
  (bind _target_position (Variables|Default|GetTarget%20Position))
  (bind _barrier_spawn_distance (Variables|Default|GetBarrier%20spawn%20distance))
  (bind _ground_line_trace_distance (LocalVariables|GetGround%20line%20trace%20distance))
  (bind (_location _rotation _scale) (Math|Transform|BreakTransform _returnvalue))
  (bind _returnvalue_2 (- _target_position _location))
  (bind _returnvalue_3 (Math|Vector|Normalize _returnvalue_2))
  (bind _returnvalue_4 (* _returnvalue_3 _barrier_spawn_distance))
  (bind _returnvalue_5 (+ _returnvalue_4 _location))
  (bind (_x _y _z) (Math|Vector|BreakVector _returnvalue_5))
  ;[1 1 1] Look for ground below
  (bind (_outhit _returnvalue_6) (Collision|LineTraceByChannel _returnvalue_5 (Math|Vector|MakeVector _x _y (- _z _ground_line_trace_distance)) "TraceTypeQuery1" false 0 "None"))
  (if _returnvalue_6
    (LocalVariables|SetSpawn%20position (.location _outhit))
    (else
      ;[1 1 1] Look for ground above
      (bind _outhit_2 (Collision|LineTraceByChannel _returnvalue_5 (Math|Vector|MakeVector _x _y (+ _z _ground_line_trace_distance)) "TraceTypeQuery1" false 0 "None"))
      (LocalVariables|SetSpawn%20position (.location _outhit_2))))
  (Game|SpawnActorfromClass "/Game/Blueprints/Spell_System/BP_Barrier.BP_Barrier_C" (Math|Transform|MakeTransform (LocalVariables|GetSpawn%20position) _rotation _scale) "AlwaysSpawn" "MultiplyWithRoot" 0 Element 0))

(fn GetElement
  (return "NewEnumerator0"))