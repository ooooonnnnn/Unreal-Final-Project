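; BP_Enemy is an enemy character Blueprint built around a cooldown-gated blink dodge.
; When moving, dodge input offsets the actor along its horizontal velocity with a sweep, triggering directional animation reaction, Niagara burst and sound.
; A timeline drives the additive reaction weight, and the cooldown toggles left and right availability particles.
; Spell casting, aiming and projectile detection are stubs that only print, trace or cast the controller.
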(event `self.ReceiveBeginPlay`
  (`|ExecutionSequence`
    (:`then_0`
      (`EnhancedInputSubsystemInterface.AddMappingContext` (subsystem `EnhancedInputLocalPlayerSubsystem`) "/Game/Input/IMC_Game.IMC_Game" 0 (struct))
      (bind _asab_abe (cast `/Game/Characters/Abe/Animation/AB_Abe` (`SkeletalMeshComponent.GetAnimInstance` (`self.Mesh`))))
      (set `self.Animation Blueprint` _asab_abe))
    (:`then_1`
      (`self.Start Dodge Cooldown`))))

(event `Event Add Dodge Input`
  (if (`self.Can Dodge`)
    (if (> (`KismetMathLibrary.VSize2DSquared` (`KismetMathLibrary.Conv_VectorToVector2D` (`CharacterMovementComponent.GetLastUpdateVelocity` (`self.CharacterMovement`)))) 0.0)
      (`|ExecutionSequence`
        (:`then_0`
          (`self.Start Dodge Cooldown`))
        (:`then_1`
          (`self.Perform Dodge`))
        (:`then_2`
          (bind (_direction _1_to_0) (`Timeline|Reaction Anim Additive Weight` :!via `PlayFromStart`)
            (:`Update`
              (`/Game/Characters/Abe/Animation/AB_Abe.Event Update Blink Additive Weight` (`self.Animation Blueprint`) _1_to_0))))))))

(event `Event On Dodge`
  (params (`Relative direction` :type "Vector2D Structure") (`World Direction` :type "Vector Structure"))
  (bind _returnvalue (`self.K2_GetActorLocation`))
  (`|ExecutionSequence`
    (:`then_0`
      (`/Game/Characters/Abe/Animation/AB_Abe.Event Blink React` (`self.Animation Blueprint`) `Relative direction`))
    (:`then_1`
      (bind _returnvalue_2 (`NiagaraFunctionLibrary.SpawnSystemAtLocation` "/Game/Niagara_Systems/NS_Star_Burst_Directional.NS_Star_Burst_Directional" _returnvalue (struct) (1.0 1.0 1.0) true false "AutoRelease"))
      (`NiagaraComponent.SetVariableVec3` _returnvalue_2 "Direction" `World Direction`)
      (`NiagaraFunctionLibrary.OverrideSystemUserVariableSkeletalMeshComponent` _returnvalue_2 "Skeletal Mesh" (`self.Mesh`))
      (`ActorComponent.Activate` _returnvalue_2 true))
    (:`then_2`
      (`GameplayStatics.PlaySoundAtLocation` "/Game/Sounds/Sound_Cues/SC_Blink.SC_Blink" _returnvalue (struct) 1.0 1.0 0.05 null null null null))))

(event `self.ProjectileDetection.OnComponentBeginOverlap`
  (params (OverlappedComponent :type "PrimitiveComponent Object Reference") (OtherActor :type "Actor Object Reference") (OtherComp :type "PrimitiveComponent Object Reference") (OtherBodyIndex :type Integer) (bFromSweep :type Boolean) (SweepResult :type "HitResult Structure (by ref)"))
  (cast `AIController` (`AIBlueprintHelperLibrary.GetAIController` self)))

(event `Event Set Aim Target Position`
  (params (`Target Position` :type "Vector Structure"))
  (`KismetSystemLibrary.LineTraceSingle` :`Start` (`self.K2_GetActorLocation`) :`End` `Target Position` :`TraceChannel` "TraceTypeQuery1" :`DrawDebugType` "ForOneFrame"))

(event `Event Cast Spell`
  (params (`Spell Data` :type "/Game/Blueprints/Structs/ST_SpellData Structure"))
  (`KismetSystemLibrary.PrintString` (`KismetTextLibrary.Conv_TextToString` (`.SpellName_14_5CB99F2D431BAB0FF0E35DBCF48975E3` (break `/Game/Blueprints/Structs/ST_SpellData` `Spell Data`)))))

(fn `Perform Dodge`
  (bind _outdir (`KismetMathLibrary.ToDirectionAndLength2D` (`KismetMathLibrary.Conv_VectorToVector2D` (`CharacterMovementComponent.GetLastUpdateVelocity` (`self.CharacterMovement`)))))
  (bind _returnvalue (`KismetMathLibrary.Conv_Vector2DToVector` (* _outdir (`self.Dodge Distance`))))
  (`self.Event On Dodge` (`KismetMathLibrary.Conv_VectorToVector2D` (`KismetMathLibrary.GreaterGreater_VectorRotator` (`KismetMathLibrary.Conv_Vector2DToVector` _outdir) (`KismetMathLibrary.FindRelativeLookAtRotation` (`self.GetTransform` self) (+ (`self.K2_GetActorLocation`) (1.0 0.0 0.0))))) (`KismetMathLibrary.Normal` _returnvalue))
  (`self.K2_AddActorWorldOffset` _returnvalue true))

(fn `UserConstructionScript`)