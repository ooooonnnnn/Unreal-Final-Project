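; Player controller that turns Enhanced Input actions into movement, camera look and dodge commands for the player's BP_Character.
; On possess it casts and caches the pawn as BP_Character, then forwards all input to that reference.
; Move input is applied along the character's own forward and right vectors, look drives controller pitch and yaw, and dodge calls the character's Dodge function.
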(event `self.ReceivePossess`
  (params (PossessedPawn :type "Pawn Object Reference"))
  (bind _asbp_character (cast `/Game/Blueprints/BP_Character` PossessedPawn))
  (set `self.Possesed Character` _asbp_character))

(event `EnhancedInput|/Game/Input/IA_Move`
  (params (ActionValue :type "Vector2D Structure") (ElapsedSeconds :type "Float (double-precision)") (TriggeredSeconds :type "Float (double-precision)") (InputAction :type "InputAction Object Reference" :default "/Game/Input/IA_Move.IA_Move"))
  (bind (_returnvalue_x _returnvalue_y) (`KismetMathLibrary.BreakVector` (`KismetMathLibrary.Conv_Vector2DToVector` ActionValue)))
  (bind _possesed_character (`self.Possesed Character`))
  (:`Triggered`
    (`Pawn.AddMovementInput` _possesed_character (+ (* (`self.GetActorRightVector` _possesed_character) _returnvalue_x) (* _returnvalue_y (`self.GetActorForwardVector` _possesed_character))) 1.0 false)))

(event `EnhancedInput|/Game/Input/IA_Look`
  (params (ActionValue :type "Vector2D Structure") (ElapsedSeconds :type "Float (double-precision)") (TriggeredSeconds :type "Float (double-precision)") (InputAction :type "InputAction Object Reference" :default "/Game/Input/IA_Look.IA_Look"))
  (bind _possesed_character (`self.Possesed Character`))
  (:`Triggered`
    (`|ExecutionSequence`
      (:`then_0`
        (bind _result (`/Engine/EditorBlueprintResources/StandardMacros.NegateFloat` ActionValue_Y)
          (:`  `
            (`Pawn.AddControllerPitchInput` _possesed_character _result))))
      (:`then_1`
        (`Pawn.AddControllerYawInput` _possesed_character ActionValue_X)))))

(event `EnhancedInput|/Game/Input/IA_Dodge`
  (params (ActionValue :type Boolean) (ElapsedSeconds :type "Float (double-precision)") (TriggeredSeconds :type "Float (double-precision)") (InputAction :type "InputAction Object Reference" :default "/Game/Input/IA_Dodge.IA_Dodge"))
  (:`Triggered`
    (`/Game/Blueprints/BP_Character.Dodge` (`self.Possesed Character`))))

(fn `UserConstructionScript`)